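; Level generator actor that builds a procedural terrain map and populates it with enemy and player ships.
; The construction script fills a height map with randomly seeded multi-octave simplex noise, then builds a procedural mesh with collision from it.
; On BeginPlay, EQS queries pick random spawn points for AI ships and, around a randomly offset helper component, the ship player 0 possesses.
; The cube generation path is unused leftover.
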(event Custom|SpawnEnemies
  (bind _returnvalue (AI|EQS|RunEQSQuery "/Game/MapGeneration/SpawnLocation.SpawnLocation" self "AllMatching"))
  (EventDispatchers|BindEventtoOnQueryFinishedEvent _returnvalue (delegate Custom|QueryFinished)))

(event Custom|QueryFinished
  (params (QueryInstance :type Env%20Query%20Instance%20Blueprint%20Wrapper%20Object%20Reference) (QueryStatus :type EEnvQueryStatus%20Enum :default "Processing"))
  (bind _returnvalue (Class|EnvQueryInstanceBlueprintWrapper|GetResultsasLocations QueryInstance))
  (for _index (range 0 3)
    (bind _returnvalue_2 (Game|SpawnActorfromClass "/Game/Ships/BaseShip/BaseShip.BaseShip_C" (Math|Transform|MakeTransform (Utilities|Array|Get(acopy) _returnvalue (Math|Random|RandomInteger (Utilities|Array|Length _returnvalue))) "0, 0, 0" "1,1,1") "Undefined" 0 0))
    (Pawn|SpawnDefaultController _returnvalue_2)))

(event Custom|GenerateMap
  (bind _scale (Variables|Default|GetScale))
  (bind _width (Variables|Default|Getwidth))
  (Class|SimplexNoiseBPLibrary|SetNoiseSeed (Math|Random|RandomIntegerinRange -5000 5000))
  (Utilities|Array|Resize (Variables|Default|GetheightMap) (* (Variables|Default|Getheight) (Variables|Default|Getwidth)))
  (if (Variables|Default|Getgenerate)
    (for _index (range 0 (Variables|Default|Getheight))
      (for _index_2 (range 0 _width)
        (Variables|Default|SetNoise 0.0)
        (Variables|Default|SetAmplitude 1.0)
        (Variables|Default|SetFrequency 1.0)
        (Utilities|FlowControl|ForLoopwithBreak 0 (Variables|Default|GetOctaves)
          (:LoopBody
            (bind _returnvalue (Class|SimplexNoiseBPLibrary|SimplexNoiseinRange2D (* (/ (Math|Conversions|ToFloat(Integer) _index_2) _scale) (Variables|Default|GetFrequency)) (* (/ (Math|Conversions|ToFloat(Integer) _index) _scale) (Variables|Default|GetFrequency)) -1.0 1.0))
            (Variables|Default|SetNoise (+ (Variables|Default|GetNoise) (* _returnvalue (Variables|Default|GetAmplitude))))
            (Variables|Default|SetFrequency (* (Variables|Default|GetFrequency) (Variables|Default|Getlacunarity)))
            (Variables|Default|SetAmplitude (* (Variables|Default|GetAmplitude) (Variables|Default|Getpersistance))))
          (:Completed
            (Utilities|Array|Insert (Variables|Default|GetheightMap) (Variables|Default|GetNoise) (+ (* _index _width) _index_2))))))
    (CallFunction|GenerateMesh)))

(event Custom|BorderQueryFinished
  (params (QueryInstance :type Env%20Query%20Instance%20Blueprint%20Wrapper%20Object%20Reference) (QueryStatus :type EEnvQueryStatus%20Enum :default "Processing"))
  (bind _returnvalue (Class|EnvQueryInstanceBlueprintWrapper|GetResultsasLocations QueryInstance))
  (bind _returnvalue_2 (Game|SpawnActorfromClass "/Game/Ships/BaseShip/BaseShip.BaseShip_C" (Math|Transform|MakeTransform (Utilities|Array|Get(acopy) _returnvalue (Math|Random|RandomInteger (Utilities|Array|Length _returnvalue))) (Math|Rotator|MakeRotator 0.0 0.0 0.0) "1,1,1") "Undefined" 0 0))
  (Pawn|Possess (Game|GetPlayerController 0) _returnvalue_2))

(event Custom|GenerateCubes
  (bind _width (Variables|Default|Getwidth))
  ;[1 1 1] Junk
  (for _index (range 0 (Variables|Default|Getheight))
    (for _index_2 (range 0 _width)
      (if (> (Utilities|Array|Get(acopy) (Variables|Default|GetheightMap) (+ _index_2 (* _index _width))) 0.0)
        (if (not (> (Utilities|Array|Get(acopy) (Variables|Default|GetheightMap) (+ _index_2 (* _index _width))) 0.2))
          (if (> (Utilities|Array|Get(acopy) (Variables|Default|GetheightMap) (+ _index_2 (* _index _width))) 0.1)
            _))))))

(event Custom|GenerateMesh
  (bind _proceduralmesh (Variables|Default|GetProceduralMesh))
  (bind _width (Variables|Default|Getwidth))
  (bind _height (Variables|Default|Getheight))
  (bind _width_2 (Variables|Default|Getwidth))
  (bind _triangles (Variables|Default|GetTriangles))
  (bind _returnvalue (+ _width_2 1))
  (Class|ProceduralMeshComponent|ClearAllMeshSections (Variables|Default|GetProceduralMesh))
  (Variables|Default|SetOffsetX (/ (* (Variables|Default|Getwidth) (Variables|Default|GetScale)) -2.0))
  (Variables|Default|SetOffsetY (/ (* (Variables|Default|Getheight) (Variables|Default|GetScale)) -2.0))
  (for _index (range 0 _height)
    (for _index_2 (range 0 _width)
      (Utilities|Array|Add (Variables|Default|GetVertices) (Math|Vector|MakeVector (+ (* (Math|Conversions|ToFloat(Integer) _index) (Variables|Default|GetScale)) (Variables|Default|GetOffsetX)) (+ (* (Math|Conversions|ToFloat(Integer) _index_2) (Variables|Default|GetScale)) (Variables|Default|GetOffsetY)) (* (Utilities|Array|Get(acopy) (Variables|Default|GetheightMap) (+ _index_2 (* _index _width))) (Variables|Default|GetheightMultiplier))))
      (Utilities|Array|Add (Variables|Default|GetUV) (Math|Vector2D|MakeVector2D (/ (Math|Conversions|ToFloat(Integer) _index_2) (Math|Conversions|ToFloat(Integer) _width)) (/ (Math|Conversions|ToFloat(Integer) _index) (Math|Conversions|ToFloat(Integer) _height))))))
  (for _index_3 (range 0 (- (Variables|Default|Getheight) 1))
    (for _index_4 (range 0 (- _width_2 1))
      (Utilities|Array|Add _triangles (+ _index_4 (* _index_3 _returnvalue)))
      (Utilities|Array|Add _triangles (+ (+ (+ _index_4 (* _index_3 _returnvalue)) _returnvalue) 1))
      (Utilities|Array|Add _triangles (+ (+ _index_4 (* _index_3 _returnvalue)) _returnvalue))
      (Utilities|Array|Add _triangles (+ _index_4 (* _index_3 _returnvalue)))
      (Utilities|Array|Add _triangles (+ (+ _index_4 (* _index_3 _returnvalue)) 1))
      (Utilities|Array|Add _triangles (+ (+ (+ _index_4 (* _index_3 _returnvalue)) 1) _returnvalue))))
  (Class|ProceduralMeshComponent|CreateMeshSectionLinearColor _proceduralmesh 0 (Variables|Default|GetVertices) (Variables|Default|GetTriangles) 0 (Variables|Default|GetUV) 0 0 true)
  (Rendering|Material|SetMaterial _proceduralmesh 0 "/Game/MapGeneration/MapMaterial.MapMaterial"))

(event Custom|SpawnPlayer
  (bind _returnvalue (Math|Random|RandomBool))
  (bind _returnvalue_2 (Math|Random|RandomBool))
  (bind _scale (Variables|Default|GetScale))
  (bind _scale_2 (Variables|Default|GetScale))
  (bind _height (Variables|Default|Getheight))
  (bind _width (Variables|Default|Getwidth))
  (bind _returnvalue_3 (/ _width 2))
  (bind _returnvalue_4 (/ _height 2))
  (bind _returnvalue_5 (select _returnvalue -1.0 1.0))
  (bind _returnvalue_6 (* _returnvalue_3 _scale_2))
  (bind _returnvalue_7 (* _returnvalue_4 _scale))
  (bind _returnvalue_8 (- _returnvalue_7 3e+02))
  (bind _returnvalue_9 (- _returnvalue_6 3e+02))
  (bind _returnvalue_10 (select _returnvalue_2 _returnvalue_8 0.0))
  (bind _returnvalue_11 (- _returnvalue_10 _returnvalue_9))
  (bind _returnvalue_12 (* _returnvalue_11 _returnvalue_5))
  (bind _returnvalue_13 (AddComponent|AddSceneComponent false (Math|Transform|MakeTransform (Math|Vector|MakeVector (* _returnvalue_10 (select (Math|Random|RandomBool) -1.0 1.0)) _returnvalue_12 0.0) (Math|Rotator|MakeRotator 0.0 0.0 (select (!= _returnvalue_12 0.0) 9e+01 0.0)))))
  (bind _returnvalue_14 (AI|EQS|RunEQSQuery "/Game/MapGeneration/BorderSpawn.BorderSpawn" _returnvalue_13 "AllMatching"))
  (EventDispatchers|BindEventtoOnQueryFinishedEvent _returnvalue_14 (delegate Custom|BorderQueryFinished)))

(event EventBeginPlay
  (CallFunction|SpawnEnemies)
  (CallFunction|Spawnplayer))

(event Collision|EventActorBeginOverlap
  (params (OtherActor :type Actor%20Object%20Reference)))

(event EventTick
  (params (DeltaSeconds :type Float%20%28single-precision%29)))

(fn ConstructionScript
  (CallFunction|GenerateMap))