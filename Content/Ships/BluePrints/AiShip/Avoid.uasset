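; AI ship behavior tree node that detects obstacles ahead and feeds steering avoidance to the ShipAIController.
; Each tick it sphere-traces forward from the controlled pawn over AvoidingDistance, using a cached controller reference.
; On a hit, flattened dot products give a steer value away from the impact side, stronger when head-on; otherwise avoidance resets.
; The alpha uses full trace length, not hit distance, so stays near one on hits.
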(event EventTick
  (params (OwnerActor :type Actor%20Object%20Reference) (DeltaSeconds :type Float%20%28single-precision%29))
  (if (!= (Variables|Default|GetAIShipContREF) 0)
    _
    (else
      (bind _asship_aicontroller (Utilities|Casting|CastToShipAIController OwnerActor))
      (Variables|Default|SetAIShipContREF _asship_aicontroller)))
  (bind (_outhit _returnvalue) (Collision|SphereTraceByChannel (Transformation|GetActorLocation (Pawn|GetControlledPawn (Variables|Default|GetAIShipContREF))) (+ (Transformation|GetActorLocation (Pawn|GetControlledPawn (Variables|Default|GetAIShipContREF))) (* (Transformation|GetActorForwardVector (Pawn|GetControlledPawn (Variables|Default|GetAIShipContREF))) (Variables|Default|GetAvoidingDistance))) 2e+01 "TraceTypeQuery3" true (Utilities|Array|MakeArray (Pawn|GetControlledPawn (Variables|Default|GetAIShipContREF))) "ForOneFrame"))
  (if _returnvalue
    (Default|SetAvoid (Variables|Default|GetAIShipContREF) (* (* (Math|Vector|DotProduct (Math|Vector|Normalize (- (Math|Vector|MakeVector (.X (Math|Vector|BreakVector (.ImpactPoint (Collision|BreakHitResult _outhit)))) (.Y (Math|Vector|BreakVector (.ImpactPoint (Collision|BreakHitResult _outhit)))) 0.0) (Math|Vector|MakeVector (.x (Transformation|GetActorLocation (Pawn|GetControlledPawn (Variables|Default|GetAIShipContREF)))) (.y (Transformation|GetActorLocation (Pawn|GetControlledPawn (Variables|Default|GetAIShipContREF)))) 0.0))) (Transformation|GetActorForwardVector (Pawn|GetControlledPawn (Variables|Default|GetAIShipContREF)))) (Math|Float|Sign(Float) (Math|Vector|DotProduct (Math|Vector|Normalize (- (Math|Vector|MakeVector (.X (Math|Vector|BreakVector (.ImpactPoint (Collision|BreakHitResult _outhit)))) (.Y (Math|Vector|BreakVector (.ImpactPoint (Collision|BreakHitResult _outhit)))) 0.0) (Math|Vector|MakeVector (.x (Transformation|GetActorLocation (Pawn|GetControlledPawn (Variables|Default|GetAIShipContREF)))) (.y (Transformation|GetActorLocation (Pawn|GetControlledPawn (Variables|Default|GetAIShipContREF)))) 0.0))) (Transformation|GetActorRightVector (Pawn|GetControlledPawn (Variables|Default|GetAIShipContREF))))) -1.0) 0.5) (/ (CallFunction|DistanceBetwen2Points (.TraceStart (Collision|BreakHitResult _outhit)) (.TraceEnd (Collision|BreakHitResult _outhit))) (Variables|Default|GetAvoidingDistance)))
    (else
      (Default|SetAvoid (Variables|Default|GetAIShipContREF) 0.0 0.0))))