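; AI ship Blueprint that automatically fires broadside cannons at targets on either side.
; Each tick it runs a left and right detector, skipping any side that is busy and both if it has no cannons.
; Each detector box-traces sideways to its first cannon's range, using a flat box sized from the mesh bounds and rotated with the ship.
; A hit on the WhatToShoot object types triggers that side's shoot call.
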(event Custom|DetectorCannL
  (bind _returnvalue (Transformation|GetActorLocation))
  (if (and (not (Variables|Default|GetLBusy)) (Variables|Default|GetHasCannons))
    (bind _returnvalue_2 (Class|KismetSystemLibrary|BoxTraceSingleforObjects _returnvalue (+ (* (Transformation|GetActorRightVector) (* (Variables|/Game/BluePrints/Cannons/Cannon.Cannon_C|GetRange (Utilities|Array|Get(acopy) (Variables|Default|GetLcannons))) -1.0)) _returnvalue) (Math|Vector|MakeVector (/ (.SphereRadius (Collision|GetComponentBounds (Variables|Default|GetStaticMesh))) 2.0) 0.0 0.0) (Transformation|GetActorRotation) (Variables|Default|GetWhatToShoot) false 0 "None" true "(R=1.000000,G=0.000000,B=0.000000,A=1.000000)" "(R=0.000000,G=1.000000,B=0.000000,A=1.000000)" 0.0))
    (if _returnvalue_2
      (CallFunction|ShootL))))

(event Custom|DetectorCannR
  (bind _returnvalue (Transformation|GetActorLocation))
  (if (and (not (Variables|Default|GetRBusy)) (Variables|Default|GetHasCannons))
    (bind _returnvalue_2 (Class|KismetSystemLibrary|BoxTraceSingleforObjects _returnvalue (+ (* (Transformation|GetActorRightVector) (Variables|/Game/BluePrints/Cannons/Cannon.Cannon_C|GetRange (Utilities|Array|Get(acopy) (Variables|Default|GetRcannons)))) _returnvalue) (Math|Vector|MakeVector (/ (.SphereRadius (Collision|GetComponentBounds (Variables|Default|GetStaticMesh))) 2.0) 0.0 0.0) (Transformation|GetActorRotation) (Variables|Default|GetWhatToShoot) false 0 "None" true "(R=0.870000,G=0.000000,B=0.000000,A=1.000000)" "(R=0.000000,G=1.000000,B=0.000000,A=1.000000)" 0.0))
    (if _returnvalue_2
      (CallFunction|ShootR))))

(event EventBeginPlay
  (|CallParentFunction))

(event Collision|EventActorBeginOverlap
  (params (OtherActor :type Actor%20Object%20Reference)))

(event EventTick
  (params (DeltaSeconds :type Float%20%28single-precision%29))
  (|CallParentFunction DeltaSeconds)
  (CallFunction|DetectorCannL)
  (CallFunction|DetectorCannR))

(fn ConstructionScript
  (|CallParentFunction))