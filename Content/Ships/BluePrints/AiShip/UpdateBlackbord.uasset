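; Behavior tree service that keeps an AI ship's Target and Position blackboard keys up to date.
; Each tick it sphere-overlaps around the controlled pawn, using a lazily cached ShipAIController, and sets the first hit as Target, clearing it if none.
; Position follows which side the target is on, switching when that side's LBusy or RBusy flag is set and staying unchanged when both are.
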(event EventTick
  (params (OwnerActor :type Actor%20Object%20Reference) (DeltaSeconds :type Float%20%28single-precision%29))
  (if (!= (Variables|Default|GetAIShipConRef) 0)
    _
    (else
      (bind _asship_aicontroller (Utilities|Casting|CastToShipAIController OwnerActor))
      (Variables|Default|SetAIShipConRef _asship_aicontroller)))
  (bind (_outactors _returnvalue) (Collision|SphereOverlapActors (Transformation|GetActorLocation (Pawn|GetControlledPawn (Variables|Default|GetAIShipConRef))) 1e+03 (Variables|Default|GetWhatToLookFor) 0 (Utilities|Array|MakeArray (Pawn|GetControlledPawn (Variables|Default|GetAIShipConRef)))))
  (if _returnvalue
    (Class|BTFunctionLibrary|SetBlackboardValueasObject (Variables|Default|GetTarget) (Utilities|Array|Get(acopy) _outactors))
    (bind _asaiship (Utilities|Casting|CastToAIShip (Pawn|GetControlledPawn (Variables|Default|GetAIShipConRef))))
    (if (Variables|/Game/BluePrints/BaseShip/BaseBoat.BaseBoat_C|GetLBusy _asaiship)
      (if (not (Variables|/Game/BluePrints/BaseShip/BaseBoat.BaseBoat_C|GetRBusy _asaiship))
        (Class|BTFunctionLibrary|SetBlackboardValueasEnum (Variables|Default|GetPosition) 1 :!label _label))
      (else
        (if (CallFunction|IsObjectonRight (Pawn|GetControlledPawn (Variables|Default|GetAIShipConRef)) (AI|BehaviorTree|GetBlackboardValueasActor (Variables|Default|GetTarget)))
          (if (Variables|/Game/BluePrints/BaseShip/BaseBoat.BaseBoat_C|GetRBusy _asaiship)
            _
            (else
              (goto _label))))
        (Class|BTFunctionLibrary|SetBlackboardValueasEnum (Variables|Default|GetPosition))))
    (else
      (Class|BTFunctionLibrary|SetBlackboardValueasObject (Variables|Default|GetTarget)))))