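; Behavior tree decorator for AI ships that passes when the blackboard Target is within a distance band from the controlled ship.
; It casts the owner to ShipAIController on first check and caches the reference.
; Each check measures the distance between the Target actor and the controlled pawn, returning true when it lies between MinDistance and MaxDistance inclusive.
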(fn PerformConditionCheck
  (params (OwnerActor :type Actor%20Object%20Reference))
  (if (!= (Variables|Default|GetAIShipContREF) 0)
    _
    (else
      (bind _asship_aicontroller (Utilities|Casting|CastToShipAIController OwnerActor))
      (Variables|Default|SetAIShipContREF _asship_aicontroller)))
  (return (and (<= (CallFunction|DistanceBetwen2Points (Transformation|GetActorLocation (AI|BehaviorTree|GetBlackboardValueasActor (Variables|Default|GetTarget))) (Transformation|GetActorLocation (Pawn|GetControlledPawn (Variables|Default|GetAIShipContREF)))) (Variables|Default|GetMaxDistance)) (>= (CallFunction|DistanceBetwen2Points (Transformation|GetActorLocation (AI|BehaviorTree|GetBlackboardValueasActor (Variables|Default|GetTarget))) (Transformation|GetActorLocation (Pawn|GetControlledPawn (Variables|Default|GetAIShipContREF)))) (Variables|Default|GetMinDistance)))))