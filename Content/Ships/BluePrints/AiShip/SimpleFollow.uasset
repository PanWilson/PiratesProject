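; Behavior tree node that makes an AI ship follow its blackboard Target at a side offset chosen by Position.
; Each tick feeds speed and turn values to the ShipAIController.
; CalculateRotation uses flattened dot products for steering and detecting a point behind the ship, which reduces speed.
; CalculateSpeed runs full throttle when far, easing exponentially toward the target boat's relative speed when close.
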(event EventTick
  (params (OwnerActor :type Actor%20Object%20Reference) (DeltaSeconds :type Float%20%28single-precision%29))
  (bind (_returnvalue _returnvalue2 _returnvalue5 _newparam) (Utilities|CalculateRotation))
  (if (!= (Variables|Default|GetShipControllerREF) 0)
    _
    (else
      (bind _asship_aicontroller (Utilities|Casting|CastToShipAIController OwnerActor))
      (bind _output_get (Variables|Default|SetShipControllerREF _asship_aicontroller))))
  (bind _returnvalue_2 (Utilities|CalculateSpeed _newparam))
  (if _returnvalue
    (Default|SetSpeed _output_get (/ _returnvalue_2 1.5))
    (else
      (Default|SetSpeed _output_get _returnvalue_2)))
  (Default|SetTurnValue _output_get _returnvalue2))