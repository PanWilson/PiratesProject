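; Behavior tree node for AI ships that steers toward the blackboard Target, or away from it when closer than the Distace threshold.
; Each tick sets full speed on the cached ShipAIController and feeds it a turn value computed on the XY plane.
; The forward-vector dot product gives clamped turn strength, and the right-vector dot product gives its sign.
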(event EventTick
  (params (OwnerActor :type Actor%20Object%20Reference) (DeltaSeconds :type Float%20%28single-precision%29))
  (bind _target (Variables|Default|GetTarget))
  (bind _returnvalue (AI|BehaviorTree|GetBlackboardValueasActor _target))
  (bind _returnvalue_2 (Transformation|GetActorLocation _returnvalue))
  (if (!= (Variables|Default|GetAIShipContREF) 0)
    _
    (else
      (bind _asship_aicontroller (Utilities|Casting|CastToShipAIController OwnerActor))
      (bind _output_get (Variables|Default|SetAIShipContREF _asship_aicontroller))))
  (Default|SetSpeed _output_get 1.0)
  (Default|SetTurnValue _output_get (* (Math|Float|Clamp(Float) (- 1.0 (Math|Vector|DotProduct (Transformation|GetActorForwardVector (Pawn|GetControlledPawn (Variables|Default|GetAIShipContREF))) (Math|Vector|Normalize (* (- (Math|Vector|MakeVector (.x _returnvalue_2) (.y _returnvalue_2) 0.0) (Math|Vector|MakeVector (.x (Transformation|GetActorLocation (Pawn|GetControlledPawn (Variables|Default|GetAIShipContREF)))) (.y (Transformation|GetActorLocation (Pawn|GetControlledPawn (Variables|Default|GetAIShipContREF)))) 0.0)) (select (>= (Transformation|GetDistanceTo (Pawn|GetControlledPawn (Variables|Default|GetAIShipContREF)) (AI|BehaviorTree|GetBlackboardValueasActor (Variables|Default|GetTarget))) (Variables|Default|GetDistace)) 1.0 -1.0))))) 0.0) (Math|Float|Sign(Float) (Math|Vector|DotProduct (Transformation|GetActorRightVector (Pawn|GetControlledPawn (Variables|Default|GetAIShipContREF))) (Math|Vector|Normalize (* (- (Math|Vector|MakeVector (.x _returnvalue_2) (.y _returnvalue_2) 0.0) (Math|Vector|MakeVector (.x (Transformation|GetActorLocation (Pawn|GetControlledPawn (Variables|Default|GetAIShipContREF)))) (.y (Transformation|GetActorLocation (Pawn|GetControlledPawn (Variables|Default|GetAIShipContREF)))) 0.0)) (select (>= (Transformation|GetDistanceTo (Pawn|GetControlledPawn (Variables|Default|GetAIShipContREF)) (AI|BehaviorTree|GetBlackboardValueasActor (Variables|Default|GetTarget))) (Variables|Default|GetDistace)) 1.0 -1.0))))))))