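; Behavior tree node that steers an AI ship to bring its left or right side to bear on the blackboard Target.
; Each tick it sets a fixed speed and a turn value on the cached ShipAIController.
; TargetPosition picks the side, and flattened dot products against the ship's forward and right vectors set turn direction and strength, easing off as that side lines up.
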(event EventTick
  (params (OwnerActor :type Actor%20Object%20Reference) (DeltaSeconds :type Float%20%28single-precision%29))
  (bind _target (Variables|Default|GetTarget))
  (bind _targetposition (Variables|Default|GetTargetPosition))
  (bind _returnvalue (Class|BTFunctionLibrary|GetBlackboardValueasEnum _targetposition))
  (bind _returnvalue_2 (AI|BehaviorTree|GetBlackboardValueasActor _target))
  (bind _returnvalue_3 (Transformation|GetActorLocation _returnvalue_2))
  (bind _returnvalue_4 (Utilities|Select :Index _returnvalue :Option%200 -1.0 :Option%201 1.0))
  (if (!= (Variables|Default|GetAIShipContREF) 0)
    _
    (else
      (bind _asship_aicontroller (Utilities|Casting|CastToShipAIController OwnerActor))
      (bind _output_get (Variables|Default|SetAIShipContREF _asship_aicontroller))))
  (Default|SetSpeed _output_get 0.8)
  (Default|SetTurnValue _output_get (* (Math|Float|Sign(Float) (Math|Vector|DotProduct (Transformation|GetActorForwardVector (Pawn|GetControlledPawn (Variables|Default|GetAIShipContREF))) (Math|Vector|Normalize (- (Math|Vector|MakeVector (.x _returnvalue_3) (.y _returnvalue_3) 0.0) (Math|Vector|MakeVector (.x (Transformation|GetActorLocation (Pawn|GetControlledPawn (Variables|Default|GetAIShipContREF)))) (.y (Transformation|GetActorLocation (Pawn|GetControlledPawn (Variables|Default|GetAIShipContREF)))) 0.0))))) (Math|Float|Clamp(Float) (- 1.0 (Math|Vector|DotProduct (* (Transformation|GetActorRightVector (Pawn|GetControlledPawn (Variables|Default|GetAIShipContREF))) _returnvalue_4) (Math|Vector|Normalize (- (Math|Vector|MakeVector (.x _returnvalue_3) (.y _returnvalue_3) 0.0) (Math|Vector|MakeVector (.x (Transformation|GetActorLocation (Pawn|GetControlledPawn (Variables|Default|GetAIShipContREF)))) (.y (Transformation|GetActorLocation (Pawn|GetControlledPawn (Variables|Default|GetAIShipContREF)))) 0.0))))) 0.0) _returnvalue_4 -1.0)))