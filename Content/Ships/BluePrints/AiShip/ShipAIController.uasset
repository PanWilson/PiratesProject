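; AI controller for ship pawns that drives them through a behavior tree.
; On BeginPlay it loads the AIShipData blackboard, runs ShipBehaviorTree and prints a debug message.
; Setter events write forward speed and turn input to the controlled AIShip.
; Turn input is eased exponentially toward a stored avoidance value by a stored alpha, so obstacle avoidance can override steering.
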(event Custom|SetTurnValue
  (params (Input :type Float%20%28single-precision%29))
  (bind _asaiship (Utilities|Casting|CastToAIShip (Pawn|GetControlledPawn)))
  (Variables|/Game/BluePrints/BaseShip/BaseBoat.BaseBoat_C|SetTurnValue _asaiship (Math|Interpolation|Ease "ExpoIn" (Variables|Default|GetAvoidingAlpha) Input (Variables|Default|GetAvoidingValue))))

(event Custom|SetSpeed
  (params (Input :type Float%20%28single-precision%29))
  (bind _asaiship (Utilities|Casting|CastToAIShip (Pawn|GetControlledPawn)))
  (Variables|/Game/BluePrints/BaseShip/BaseBoat.BaseBoat_C|SetForwardValue _asaiship Input))

(event Custom|SetAvoid
  (params (Value :type Float%20%28single-precision%29) (Alpha :type Float%20%28single-precision%29))
  (Variables|Default|SetAvoidingValue Value)
  (Variables|Default|SetAvoidingAlpha Alpha))

(event EventBeginPlay
  (Class|AIController|UseBlackboard "/Game/BluePrints/AiShip/AIShipData.AIShipData")
  (AI|RunBehaviorTree "/Game/BluePrints/AiShip/ShipBehaviorTree.ShipBehaviorTree")
  (Development|PrintString "TreeRunning" true true "(R=1.000000,G=0.000000,B=0.929469,A=1.000000)" 6e+01))

(event EventTick
  (params (DeltaSeconds :type Float%20%28single-precision%29)))

(fn ConstructionScript)