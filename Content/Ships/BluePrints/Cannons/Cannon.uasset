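; Ship cannon Blueprint that fires a projectile of its ammunition class when its Shoot event is called.
; After a short random delay, it spawns the projectile at the mesh transform, passing along the Instigator.
; For CannonBall projectiles, it solves launch speed from Range, Degree and gravity using the ballistic range formula, adding random spread to pitch, yaw and range.
; It then plays an explosion sound at random pitch.
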(event Custom|Shoot
  (params (Instigator :type Pawn%20Object%20Reference))
  (bind _audio (Variables|Default|GetAudio))
  (bind _degree (Variables|Default|GetDegree))
  (Utilities|FlowControl|Delay (Math|Random|RandomFloatinRange 0.0 0.3))
  (bind _returnvalue (Game|SpawnActorfromClass (Variables|Default|GetAmmunitionClass) (Transformation|GetWorldTransform (Variables|Default|GetStaticMesh)) "Undefined" 0 Instigator))
  (bind _ascannon_ball (Utilities|Casting|CastToCannonBall _returnvalue))
  (Game|Components|ProjectileMovement|SetVelocityinLocalSpace (Variables|/Game/BluePrints/Cannons/CannonBall.CannonBall_C|GetProjectileMovement _ascannon_ball) (* (Math|Rotator|GetRotationXVector (Math|Rotator|MakeRotator 0.0 (+ _degree (Math|Random|RandomFloatinRange -3.0 3.0)) (Math|Random|RandomFloatinRange -5.0 5.0))) (Math|Float|Sqrt (/ (* (Math|Float|Absolute(Float) (Components|Movement|GetGravityZ (Variables|/Game/BluePrints/Cannons/CannonBall.CannonBall_C|GetProjectileMovement _ascannon_ball))) (+ (Variables|Default|GetRange) (Math|Random|RandomFloatinRange -1e+01 1e+01))) (Math|Trig|Sin(Degrees) (* _degree 2.0))))))
  (Audio|Components|Audio|SetSound _audio "/Game/Audio/Explosion02.Explosion02")
  (Audio|Components|Audio|SetPitchMultiplier _audio (Math|Random|RandomFloatinRange 0.5 1.5))
  (Audio|Components|Audio|Play _audio 0.0))

(fn ConstructionScript)