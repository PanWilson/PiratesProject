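; Base boat with physics-driven sailing, broadside cannons and health shown on a text label.
; While given forward input, Tick applies thrust, curve-scaled turning torque and a sideways anti-slide force to the Box, using frame-measured speed.
; BeginPlay spawns cannons at mesh sockets, grouped by L/R name prefix (left by default), each side firing behind a DoOnce reload delay.
; Damage lowers health, disabling movement at zero.
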(event Custom|GoForward
  (bind _box (Variables|Default|GetBox))
  ;[1 1 1] Movement
  (if (< (Variables|Stats|GetSpeed) (* (Variables|Movement|GetMaxSpeed) (Variables|Movement|GetForwardValue)))
    (Physics|AddForce _box (* (Math|Vector|GetForwardVector _box) (Variables|Movement|GetAcceleration)) "None" true)))

(event Custom|Turn
  (bind _box (Variables|Default|GetBox))
  ;[1 1 1] Movement
  (Class|PrimitiveComponent|AddTorque _box (* (Math|Vector|GetUpVector _box) (* (Variables|Movement|GetTurnRate) (Variables|Movement|GetTurnValue) (Math|Curves|GetFloatValue (Variables|Movement|GetTurnToSpeedCurve) (/ (Variables|Stats|GetSpeed) (Variables|Movement|GetMaxSpeed))))) "None" true))

(event Custom|ShootR
  ;[1 1 1] Shooting
  (Utilities|FlowControl|DoOnce false
    (:Completed
      (for _array_element (Variables|Cannons|GetRcannons)
        (Default|Shoot _array_element self)
        (Variables|Default|SetRBusy true)
        (Utilities|FlowControl|Delay (Variables|Cannons|GetReloadTimeR))
        (Variables|Default|SetRBusy false)
        (CallFunction|ReloadR)))))

(event Custom|ShootL
  ;[1 1 1] Shooting
  (Utilities|FlowControl|DoOnce false
    (:Completed
      (for _array_element (Variables|Cannons|GetLcannons)
        (Default|Shoot _array_element self)
        (Variables|Default|SetLBusy true)
        (Utilities|FlowControl|Delay (Variables|Cannons|GetReloadTimeL))
        (Variables|Default|SetLBusy false)
        (CallFunction|ReloadL)))))

(event Custom|AntiSlide
  (bind _box (Variables|Default|GetBox))
  ;[1 1 1] AntiSlide
  (if (> (Variables|Stats|GetSpeed) 5e+01)
    (Physics|AddForce _box (* (Math|Vector|GetRightVector _box) (* (Variables|Movement|GetRightDeviation) (Variables|Movement|GetAntiSlidingForce) -1.0)) "None" true)))

(event Custom|ReloadL
  ;[1 1 1] Shooting
  (Utilities|FlowControl|DoOnce false) ; enters at Reset
)

(event Custom|ReloadR
  ;[1 1 1] Shooting
  (Utilities|FlowControl|DoOnce false) ; enters at Reset
)

(event EventBeginPlay
  ;[1 1 1] Begin Play
  (Variables|Default|SetLastFramePosition (Transformation|GetWorldLocation (Variables|Default|GetBox)))
  (Utilities|CannonLogic
    (:out
      (Rendering|Components|TextRender|SetText (Variables|Default|GetTextRender) (Utilities|Text|ToText(Float) (Variables|Default|GetHealth) "HalfToEven")))))

(event EventTick
  (params (DeltaSeconds :type Float%20%28single-precision%29))
  ;[1 1 1] Tick
  (Variables|Stats|SetDeltaSec DeltaSeconds)
  (Utilities|FlowControl|Sequence
    (:then_0
      (Variables|Stats|SetSpeed (Utilities|CalculateSpeed))
      (Variables|Default|SetLastFramePosition (Transformation|GetWorldLocation (Variables|Default|GetBox))))
    (:then_1
      (if (and (> (Variables|Movement|GetForwardValue) 0.0) (Variables|Default|GetMovementEnabled))
        (Variables|Movement|SetRightDeviation (Utilities|CalculateRightDeviation))
        (CallFunction|GoForward)
        (CallFunction|Turn)
        (CallFunction|AntiSlide)))))

(event Game|Damage|EventAnyDamage
  (params (Damage :type Float%20%28single-precision%29) (DamageType :type Damage%20Type%20Object%20Reference) (InstigatedBy :type Controller%20Object%20Reference) (DamageCauser :type Actor%20Object%20Reference))
  (Development|PrintString (Utilities|String|Append (Utilities|String|BuildString(Float) (Utilities|GetDisplayName self) " Got " Damage "  DMG") " From " (Utilities|GetDisplayName DamageCauser)) true true "(R=1.000000,G=0.022204,B=0.000000,A=1.000000)")
  (if (Variables|Actor|GetbCanBeDamaged)
    (bind _output_get (Variables|Default|SetHealth (- (Variables|Default|GetHealth) Damage)))
    (Rendering|Components|TextRender|SetText (Variables|Default|GetTextRender) (Utilities|Text|ToText(Float) _output_get "HalfToEven"))
    (if (<= _output_get 0.0)
      (Variables|Default|SetMovementEnabled false)
      (Development|PrintString (Utilities|String|Append (Utilities|GetDisplayName self) " DEAD") true true "(R=1.000000,G=0.811676,B=0.000000,A=1.000000)"))))

(fn ConstructionScript)